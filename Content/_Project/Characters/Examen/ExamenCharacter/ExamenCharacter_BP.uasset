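; ExamenCharacter_BP is a playable character Blueprint with glide, jet jump and bomb skills.
; On BeginPlay it initializes health, armor and shield, then initializes each skill component with itself and a key label and adds it to Skills.
; Input actions delegate to the skills: Jump fires and finishes the glide, Skill_0 fires the jet jump, and Skill_1 fires the bomb from the SpawnBulletsPoint transform.
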(event `self.ReceiveBeginPlay`
  (bind _jetjump_skill_bp (`self.JetJump_Skill_BP`))
  (bind _bomb_bp (`self.Bomb_BP`))
  (bind _glide_skill_bp (`self.Glide_Skill_BP`))
  (`parent.ReceiveBeginPlay`)
  (`|ExecutionSequence`
    (:`then_0`
      (`self.InitializeHealth` (make `/Game/_Project/CommonSystems/HealthSystem/HealthData` 200.0 200.0 50.0 50.0 50.0 50.0)))
    (:`then_1`
      (`/Game/_Project/CommonSystems/Character_Skills/Character_Skill_BP.Initialize` _glide_skill_bp self "SPACE")
      (`KismetArrayLibrary.Array_Add` (`self.Skills`) _glide_skill_bp))
    (:`then_2`
      (`/Game/_Project/CommonSystems/Character_Skills/Character_Skill_BP.Initialize` _jetjump_skill_bp self "SHIFT")
      (`KismetArrayLibrary.Array_Add` (`self.Skills`) _jetjump_skill_bp))
    (:`then_3`
      (`/Game/_Project/CommonSystems/Character_Skills/Character_Skill_BP.Initialize` _bomb_bp self "E")
      (`KismetArrayLibrary.Array_Add` (`self.Skills`) _bomb_bp))))

(event `EnhancedInput|/Game/_Project/CommonSystems/Input/Jump`
  (params (ActionValue :type Boolean) (ElapsedSeconds :type "Float (double-precision)") (TriggeredSeconds :type "Float (double-precision)") (InputAction :type "InputAction Object Reference" :default "/Game/_Project/CommonSystems/Input/Jump.Jump"))
  (bind _glide_skill_bp (`self.Glide_Skill_BP`))
  (:`Triggered`
    (`/Game/_Project/CommonSystems/Character_Skills/Character_Skill_BP.Fire` _glide_skill_bp :!label _label))
  (:`Started`
    (goto _label))
  (:`Canceled`
    (`/Game/_Project/CommonSystems/Character_Skills/Character_Skill_BP.Finish` _glide_skill_bp :!label _label_2))
  (:`Completed`
    (goto _label_2)))

(event `EnhancedInput|/Game/_Project/CommonSystems/Input/Skill_0`
  (params (ActionValue :type Boolean) (ElapsedSeconds :type "Float (double-precision)") (TriggeredSeconds :type "Float (double-precision)") (InputAction :type "InputAction Object Reference" :default "/Game/_Project/CommonSystems/Input/Skill_0.Skill_0"))
  (:`Triggered`
    (`/Game/_Project/CommonSystems/Character_Skills/Character_Skill_BP.Fire` (`self.JetJump_Skill_BP`) :!label _label_3))
  (:`Started`
    (goto _label_3)))

(event `EnhancedInput|/Game/_Project/CommonSystems/Input/Skill_1`
  (params (ActionValue :type Boolean) (ElapsedSeconds :type "Float (double-precision)") (TriggeredSeconds :type "Float (double-precision)") (InputAction :type "InputAction Object Reference" :default "/Game/_Project/CommonSystems/Input/Skill_1.Skill_1"))
  (bind _bomb_bp (`self.Bomb_BP`))
  (:`Triggered`
    (set `/Game/_Project/Characters/Examen/Skills/Bomb/Bomb_BP.SpawnPoint` (`SceneComponent.K2_GetComponentToWorld` (`self.SpawnBulletsPoint`)) _bomb_bp)
    (`/Game/_Project/CommonSystems/Character_Skills/Character_Skill_BP.Fire` _bomb_bp)))

(fn `UserConstructionScript`
  (`parent.UserConstructionScript`))