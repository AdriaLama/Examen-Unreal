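; Bomb skill Blueprint for the Examen character that launches a grenade when fired.
; Fire runs the parent logic, then, in one specific State, spawns a Bomb_BP_Grenade at SpawnPoint whose Bomb component ignores the owning character when moving.
; It then calls Finish if its own Bomb reference is invalid.
; The node assigning the grenade's OwningCharacter is disconnected and never runs.
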(event `self.Fire`
  (`parent.Fire`)
  (if (`|EnumEquality` (`self.State`) "NewEnumerator1")
    (bind _returnvalue (`|SpawnActorFromClass` "/Game/_Project/Characters/Examen/Skills/Bomb/Bomb_BP_Grenade.Bomb_BP_Grenade_C" (`self.SpawnPoint`) "Undefined" "MultiplyWithRoot" null null))
    (`|ExecutionSequence`
      (:`then_0`
        (`PrimitiveComponent.IgnoreActorWhenMoving` (`/Game/_Project/Characters/Examen/Skills/Bomb/Bomb_BP_Grenade.Bomb` _returnvalue) (`self.OwningCharacter`) true)
        (`/Engine/EditorBlueprintResources/StandardMacros.IsValid` (`self.bomb`)
          (:`Is Not Valid`
            (`self.Finish`)))))))