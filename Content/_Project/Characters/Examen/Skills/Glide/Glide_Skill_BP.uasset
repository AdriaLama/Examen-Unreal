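; Glide skill Blueprint, derived from a parent skill, that slows the owning character's fall while Jump is held in midair.
; Jump input tracks the held state; Tick switches the skill state, caps descent speed through a Z-override LaunchCharacter and raises air control.
; Otherwise Tick restores the state and low air control, but never clears IsGliding.
; Fire calls the parent and activates the skill UI when enabled.
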(event `self.Initialize`
  (params (OwningCharacter :type "/Game/_Project/Characters/BaseCharacter_BP Object Reference") (`Control Text` :type String))
  (`parent.Initialize` OwningCharacter `Control Text`))

(event `self.ReceiveTick`
  (params (DeltaSeconds :type "Float (single-precision)"))
  (`parent.ReceiveTick` DeltaSeconds)
  (if (and (`NavMovementComponent.IsFalling` (`Character.CharacterMovement` (`self.OwningCharacter`))) (`self.isSpaceHeld`))
    (set `self.State` "NewEnumerator1")
    (set `self.isGliding` true)
    (if (< (.z (`Actor.GetVelocity` (`self.OwningCharacter`))) -200.0)
      (`Character.LaunchCharacter` (`self.OwningCharacter`) (0.0 0.0 -200.0) false true)
      (set `CharacterMovementComponent.AirControl` 0.5 (`Character.CharacterMovement` (`self.OwningCharacter`))))
    (else
      (set `self.State` "NewEnumerator0")
      (set `CharacterMovementComponent.AirControl` 0.05 (`Character.CharacterMovement` (`self.OwningCharacter`))))))

(event `EnhancedInput|/Game/_Project/CommonSystems/Input/Jump`
  (params (ActionValue :type Boolean) (ElapsedSeconds :type "Float (double-precision)") (TriggeredSeconds :type "Float (double-precision)") (InputAction :type "InputAction Object Reference" :default "/Game/_Project/CommonSystems/Input/Jump.Jump"))
  (:`Triggered`
    (set `self.isSpaceHeld` true))
  (:`Completed`
    (set `self.isSpaceHeld` false)))

(event `self.Fire`
  (`parent.Fire`)
  (if (`self.Enabled`)
    (`/Game/_Project/CommonSystems/Character_UI/BaseUI/Skill/SkillUI.SetActive` (`self.UI`) true)))