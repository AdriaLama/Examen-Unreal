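; Ultimate skill for the Examen character that is meant to rewind its owner along recorded positions, apparently unfinished.
; A timer event set on BeginPlay stores the owner's transform at the front of a resized history array while not recalling.
; Left Shift starts recall, stopping movement and disabling input, with no reset here.
; Tick sets transforms without checking recall state; its interpolation branch is unreachable, and recall time never advances here.
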(event `self.ReceiveBeginPlay`
  (`parent.ReceiveBeginPlay`)
  (`KismetSystemLibrary.K2_SetTimerDelegate` (delegate `CustomEvent`)))

(event `CustomEvent`
  (if (not (`self.isRecalling`))
    (`KismetArrayLibrary.Array_Insert` (`self.RecallPos`) (`Actor.GetTransform` (`self.OwningCharacter`)))
    (`KismetArrayLibrary.Array_Resize` (`self.RecallPos`) (`KismetMathLibrary.Round` (/ (`self.CurrentRecallTime`) (`self.MaxRecallTime`))))))

(event `Key|LeftShift`
  (params (Key :type "Key Structure"))
  (:`Pressed`
    (set `self.isRecalling` true)
    (`MovementComponent.StopMovementImmediately` (`Character.CharacterMovement` (`self.OwningCharacter`)))
    (`Actor.DisableInput` (`self.OwningCharacter`) (`PlayerState.GetPlayerController` (`Pawn.PlayerState` (`self.OwningCharacter`))))))

(event `self.ReceiveTick`
  (params (DeltaSeconds :type "Float (single-precision)"))
  (bind _recallpos (`self.RecallPos`))
  (bind _recallpos_2 (`self.RecallPos`))
  (bind _returnvalue (`KismetArrayLibrary.Array_Length` _recallpos_2))
  (bind _returnvalue_2 (`KismetMathLibrary.FFloor` (/ (`self.CurrentRecallTime`) (`self.RecallSafeTime`))))
  (`parent.ReceiveTick` DeltaSeconds)
  (if (== _returnvalue_2 _returnvalue)
    (if true
      (`Actor.K2_SetActorTransform` (`self.OwningCharacter`) (`|GetArrayItem` _recallpos_2 _returnvalue) false false)
      (else
        (`Actor.K2_SetActorTransform` (`self.OwningCharacter`) (`KismetMathLibrary.TLerp` (`|GetArrayItem` _recallpos _returnvalue_2) (`|GetArrayItem` _recallpos (+ _returnvalue_2 1)) (mod (`self.CurrentRecallTime`) (`self.RecallSafeTime`))) false false)))))