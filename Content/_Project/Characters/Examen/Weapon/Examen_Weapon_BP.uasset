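; Child weapon Blueprint that fires Bullet_BP projectiles from the owning ExamenCharacter_BP's spawn point in two modes.
; Primary Fire shoots a timed three-round burst, with each bullet ignoring and recording its owner, then calling parent Fire and entering cooldown.
; SecondaryFire input is gated by weapon State and launches a simultaneous three-way yaw spread, then enters cooldown after a delay.
; Unlike burst bullets, spread bullets get no owner or ignore setup.
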(event `self.Fire`
  (`self.ShootingBullets`)
  (`KismetSystemLibrary.Delay` 0.33)
  (`self.ShootingBullets`)
  (`KismetSystemLibrary.Delay` 0.33)
  (`self.ShootingBullets`))

(event `ShootingBullets`
  (`|ExecutionSequence`
    (:`then_0`
      (bind _returnvalue (`|SpawnActorFromClass` "/Game/_Project/Characters/Examen/Weapon/Bullet_BP.Bullet_BP_C" (`SceneComponent.K2_GetComponentToWorld` (`/Game/_Project/Characters/Examen/ExamenCharacter/ExamenCharacter_BP.SpawnBulletsPoint` (cast `/Game/_Project/Characters/Examen/ExamenCharacter/ExamenCharacter_BP` (`self.OwningCharacter`) :!pure true))) "Undefined" "MultiplyWithRoot" null null))
      (`|ExecutionSequence`
        (:`then_0`
          (`PrimitiveComponent.IgnoreActorWhenMoving` (`/Game/_Project/Characters/Examen/Weapon/Bullet_BP.Bullet` _returnvalue) (`self.OwningCharacter`) true))
        (:`then_1`
          (set `/Game/_Project/Characters/Examen/Weapon/Bullet_BP.OwningCharacter` (`self.OwningCharacter`) _returnvalue))))
    (:`then_1`
      (`parent.Fire`))
    (:`then_2`
      (`self.EnterFireCooldown`))))

(event `EnhancedInput|/Game/_Project/CommonSystems/Input/SecondaryFire`
  (params (ActionValue :type Boolean) (ElapsedSeconds :type "Float (double-precision)") (TriggeredSeconds :type "Float (double-precision)") (InputAction :type "InputAction Object Reference" :default "/Game/_Project/CommonSystems/Input/SecondaryFire.SecondaryFire"))
  (:`Triggered`
    (if (`|EnumEquality` (`self.State`) "NewEnumerator0")
      (set `self.State` "NewEnumerator1")
      (`|ExecutionSequence`
        (:`then_0`
          (`self.ShootDirectional` (struct :`Yaw` 15.0)))
        (:`then_1`
          (`self.ShootDirectional` (struct)))
        (:`then_2`
          (`self.ShootDirectional` (struct :`Yaw` -15.0)))
        (:`then_3`
          (`KismetSystemLibrary.Delay` 0.5)
          (`self.EnterFireCooldown`))))))

(event `ShootDirectional`
  (params (DirOffset :type "Rotator Structure"))
  (`parent.Fire`)
  (`|SpawnActorFromClass` "/Game/_Project/Characters/Examen/Weapon/Bullet_BP.Bullet_BP_C" (`KismetMathLibrary.MakeTransform` (.location (`SceneComponent.K2_GetComponentToWorld` (`/Game/_Project/Characters/Examen/ExamenCharacter/ExamenCharacter_BP.SpawnBulletsPoint` (cast `/Game/_Project/Characters/Examen/ExamenCharacter/ExamenCharacter_BP` (`self.OwningCharacter`) :!pure true)))) (`KismetMathLibrary.MakeRotator` (.roll (.rotation (`SceneComponent.K2_GetComponentToWorld` (`/Game/_Project/Characters/Examen/ExamenCharacter/ExamenCharacter_BP.SpawnBulletsPoint` (cast `/Game/_Project/Characters/Examen/ExamenCharacter/ExamenCharacter_BP` (`self.OwningCharacter`) :!pure true))))) (.pitch (.rotation (`SceneComponent.K2_GetComponentToWorld` (`/Game/_Project/Characters/Examen/ExamenCharacter/ExamenCharacter_BP.SpawnBulletsPoint` (cast `/Game/_Project/Characters/Examen/ExamenCharacter/ExamenCharacter_BP` (`self.OwningCharacter`) :!pure true))))) (+ (.yaw (.rotation (`SceneComponent.K2_GetComponentToWorld` (`/Game/_Project/Characters/Examen/ExamenCharacter/ExamenCharacter_BP.SpawnBulletsPoint` (cast `/Game/_Project/Characters/Examen/ExamenCharacter/ExamenCharacter_BP` (`self.OwningCharacter`) :!pure true))))) (.yaw DirOffset))) (.scale (`SceneComponent.K2_GetComponentToWorld` (`/Game/_Project/Characters/Examen/ExamenCharacter/ExamenCharacter_BP.SpawnBulletsPoint` (cast `/Game/_Project/Characters/Examen/ExamenCharacter/ExamenCharacter_BP` (`self.OwningCharacter`) :!pure true))))) "Undefined" "MultiplyWithRoot" null null))